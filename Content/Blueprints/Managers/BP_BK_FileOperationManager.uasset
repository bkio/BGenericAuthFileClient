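; Manager that runs upload, download, delete and cancel operations for model version files, reporting through events and notifications.
; Maps link action and file IDs to progress and cancellation tokens, letting users or lost authentication kill active transfers.
; Uploads rejected as Bad Request delete the file and upload again.
; After uploads and deletes, a tick enabled only while checks are pending polls version info until the expected stage or retries run out.
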(event `OnPerformUploadRawFile_Internal`
  (params (FileInput :type "BKActionUploadRawFileInput Structure"))
  (bind (_modelid _revisionindex _versionindex _fileentryname _filepaths _topassemblynameifany _potentialcadsoftwarenames) (break `BKActionUploadRawFileInput` FileInput))
  (bind (_modelid_2 _revisionindex_2 _versionindex_2) (break `BKActionUploadRawFileInput` FileInput))
  (bind _returnvalue (`BKActionBlueprintFunctionLibrary.MakeFileId` _modelid_2 _revisionindex_2 _versionindex_2))
  ;[1 1 1] Upload File
  ;;[1 1 1] Perform upload action
  ;;;[1 1 1] Create and store Cancellation Token and Action Id
  (bind _returnvalue_2 (`|GenericCreateObject` "/BGenericAuthFileSrvClient/Blueprints/BP_BK_EmptyCancellationTokenObject.BP_BK_EmptyCancellationTokenObject_C" self))
  (`/BGenericAuthFileSrvClient/Blueprints/BP_BK_EmptyCancellationTokenObject.SetRelevantToken` _returnvalue_2 (`BKCancellationToken.MakeFromUObject` _returnvalue_2))
  (bind _output (`/BGenericAuthFileSrvClient/Blueprints/BP_BK_EmptyCancellationTokenObject.SetRelevantToken` _returnvalue_2 (`BKCancellationToken.MakeFromUObject` _returnvalue_2)))
  (`BlueprintMapLibrary.Map_Add` (`self.FileIdCancellationTokenObjectMap`) _returnvalue _returnvalue_2)
  (bind _returnvalue_3 (`BKActionBase.GenerateActionId`))
  (`BlueprintMapLibrary.Map_Add` (`self.ActionIdFileId`) _returnvalue_3 _returnvalue)
  (bind _output_2 (`BKActionUploadRawFile.Perform_UploadRawFile_Action_BP` (make `BKActionUploadRawFileInput` _modelid _revisionindex _versionindex _fileentryname _filepaths _topassemblynameifany _potentialcadsoftwarenames _returnvalue_3 true _output))
    (:`OnProgress`
      (bind (_relativeinput _progress _message _errorcode) (break `BKActionUploadRawFileOutput` _output_2))
      (bind (_value _returnvalue_4) (`BlueprintMapLibrary.Map_Find` (`self.ActionIdFileId`) (`.ActionId` (break `BKActionUploadRawFileInput` _relativeinput))))
      ;;;[0 1 0.007843] Update progress
      (if _returnvalue_4
        (`self.OnUpdateProgress` _value _progress)))
    (:`Succeed`
      ;;;[0 1 0.007843] Succeeded
      (`BKNotificationManager.SendNotification` (`BKManagerStore.GetNotificationManager`) _message 4.0)
      (bind _returnvalue_5 (`BKActionBlueprintFunctionLibrary.MakeFileId` (break `BKActionUploadRawFileInput` _relativeinput) (`.RevisionIndex` (break `BKActionUploadRawFileInput` _relativeinput)) (`.VersionIndex` (break `BKActionUploadRawFileInput` _relativeinput))))
      (`self.OnUploadFileSucceeded` _returnvalue_5)
      (`self.Add File for Retry State` _returnvalue_5 1)
      (`BlueprintMapLibrary.Map_Remove` (`self.ActionIdFileId`) (`.ActionId` (break `BKActionUploadRawFileInput` _relativeinput)) :!label _label)
      (`BlueprintMapLibrary.Map_Remove` (`self.FileIdCancellationTokenObjectMap`) _returnvalue_5))
    (:`Failed`
      ;;;[1 0 0.1221] Upload files failed
      (`self.OnFileProgressFailed` _returnvalue_5)
      (switch `EBKActionErrorCode` _errorcode
        (:`BadRequest`
          (bind _relativeinput_2 (break `BKActionUploadRawFileOutput` _output_2))
          (`self.OnDeleteFile` (break `BKActionUploadRawFileInput` _relativeinput_2) (`.RevisionIndex` (break `BKActionUploadRawFileInput` _relativeinput_2)) (`.VersionIndex` (break `BKActionUploadRawFileInput` _relativeinput_2)))
          (`BlueprintMapLibrary.Map_Remove` (`self.ActionIdFileId`) (`.ActionId` (break `BKActionUploadRawFileInput` _relativeinput)))
          (`BlueprintMapLibrary.Map_Remove` (`self.FileIdCancellationTokenObjectMap`) _returnvalue_5)
          (`self.OnPerformUploadRawFile_Internal` (make `BKActionUploadRawFileInput` (break `BKActionUploadRawFileInput` _relativeinput_2) (`.RevisionIndex` (break `BKActionUploadRawFileInput` _relativeinput_2)) (`.VersionIndex` (break `BKActionUploadRawFileInput` _relativeinput_2)) (`.FileEntryName` (break `BKActionUploadRawFileInput` _relativeinput_2)) (`.FilePaths` (break `BKActionUploadRawFileInput` _relativeinput_2)) (`.TopAssemblyNameIfAny` (break `BKActionUploadRawFileInput` _relativeinput_2)) (`.PotentialCADSoftwareNames` (break `BKActionUploadRawFileInput` _relativeinput_2)))))))
    (:`Canceled`
      ;;;[1 0 0.09412] Upload Cancelled by user
      (`self.OnUpdateProgressCancelled` _returnvalue_5)
      (goto _label))))

(event `OnUploadFile`
  (params (DialogType :type "EBDialogType Enum" :default "FilesForUpload") (ModelId :type String) (RevisionIndex :type Integer) (VersionIndex :type Integer))
  ;[1 1 1] Upload File
  ;;[1 1 1] Filepicker
  (bind _returnvalue (`|GenericCreateObject` "/BGenericAuthFileSrvClient/Blueprints/BP_BK_EmptyCancellationTokenObject.BP_BK_EmptyCancellationTokenObject_C" self))
  (bind _output (`/BGenericAuthFileSrvClient/Blueprints/BP_BK_EmptyCancellationTokenObject.SetRelevantToken` _returnvalue (`BKCancellationToken.MakeFromUObject` _returnvalue)))
  (bind _returnvalue_2 (`BKActionBase.GenerateActionId`))
  (bind _output_2 (`BKActionSelectLocalRawFiles.Perform_Select_Local_Raw_Files_Action_BP` (make `BKActionSelectLocalRawFilesInput` DialogType _returnvalue_2 true _output))
    (:`Succeed`
      (bind (_relativeinput _errormessage _selectedfilepaths _topassemblyfilenameifany _potentialcadsoftwarenames _fileentryname) (break `BKActionSelectLocalRawFilesOutput` _output_2))
      (`self.OnPerformUploadRawFile_Internal` (make `BKActionUploadRawFileInput` ModelId RevisionIndex VersionIndex _fileentryname _selectedfilepaths _topassemblyfilenameifany _potentialcadsoftwarenames)))
    (:`Failed`
      ;;;[1 1 1] Filepicker failed
      (`BKNotificationManager.SendNotification` (`BKManagerStore.GetNotificationManager`) _errormessage 4.0))))

(event `OnDownloadFile`
  (params (ModelId :type String) (RevisionIndex :type Integer) (VersionIndex :type Integer))
  (bind _returnvalue (`BKActionBlueprintFunctionLibrary.MakeFileId` ModelId RevisionIndex VersionIndex))
  ;[1 1 1] Download file
  ;;[1 1 1] File picker
  (bind _returnvalue_2 (`|GenericCreateObject` "/BGenericAuthFileSrvClient/Blueprints/BP_BK_EmptyCancellationTokenObject.BP_BK_EmptyCancellationTokenObject_C" self))
  (bind _output (`/BGenericAuthFileSrvClient/Blueprints/BP_BK_EmptyCancellationTokenObject.SetRelevantToken` _returnvalue_2 (`BKCancellationToken.MakeFromUObject` _returnvalue_2)))
  (bind _returnvalue_3 (`BKActionBase.GenerateActionId`))
  (bind _output_2 (`BKActionSelectLocalRawFiles.Perform_Select_Local_Raw_Files_Action_BP` (make `BKActionSelectLocalRawFilesInput` "FilesForUpload" _returnvalue_3 false _output))
    (:`Succeed`
      ;;[1 1 1] Perform download action
      ;;;[1 1 1] Create and store Cancellation Token and Action Id
      (bind _returnvalue_4 (`|GenericCreateObject` "/BGenericAuthFileSrvClient/Blueprints/BP_BK_EmptyCancellationTokenObject.BP_BK_EmptyCancellationTokenObject_C" self))
      (bind _output_3 (`/BGenericAuthFileSrvClient/Blueprints/BP_BK_EmptyCancellationTokenObject.SetRelevantToken` _returnvalue_4 (`BKCancellationToken.MakeFromUObject` _returnvalue_4)))
      (`BlueprintMapLibrary.Map_Add` (`self.FileIdCancellationTokenObjectMap`) _returnvalue _returnvalue_4)
      (bind _returnvalue_5 (`BKActionBase.GenerateActionId`))
      (`BlueprintMapLibrary.Map_Add` (`self.ActionIdFileId`) _returnvalue_5 _returnvalue)
      (bind (_relativeinput _errormessage _selectedfilepaths _topassemblyfilenameifany _potentialcadsoftwarenames _fileentryname _selecteddirectorypath) (break `BKActionSelectLocalRawFilesOutput` _output_2))
      (bind _output_4 (`BKActionDownloadRawFile.Perform_DownloadRawFile_Action_BP` (make `BKActionDownloadRawFileInput` ModelId RevisionIndex VersionIndex (`KismetStringLibrary.Concat_StrStr` _selecteddirectorypath _fileentryname ".zip") _returnvalue_5 true _output_3))
        (:`OnProgress`
          (bind (_relativeinput_2 _progress _message) (break `BKActionDownloadRawFileOutput` _output_4))
          (bind (_modelid _revisionindex _versionindex _destinationlocalpath _actionid) (break `BKActionDownloadRawFileInput` _relativeinput_2))
          ;;;[0 1 0.007843] Update progress
          (`self.OnUpdateProgress` (`BlueprintMapLibrary.Map_Find` (`self.ActionIdFileId`) _actionid) _progress))
        (:`Succeed`
          ;;;[0 1 0.007843] Succeeded
          (`BKNotificationManager.SendNotification` (`BKManagerStore.GetNotificationManager`) _message 4.0)
          (bind _returnvalue_6 (`BKActionBlueprintFunctionLibrary.MakeFileId` _modelid _revisionindex _versionindex))
          (`self.OnDownloadFileSucceeded` _returnvalue_6)
          (`BlueprintMapLibrary.Map_Remove` (`self.FileIdCancellationTokenObjectMap`) _returnvalue_6 :!label _label_2)
          (`BlueprintMapLibrary.Map_Remove` (`self.ActionIdFileId`) _actionid))
        (:`Failed`
          ;;;[1 0 0.09412] Download failed
          (`self.OnFileProgressFailed` (`BlueprintMapLibrary.Map_Find` (`self.ActionIdFileId`) _actionid))
          (`BKNotificationManager.SendNotification` (`BKManagerStore.GetNotificationManager`) (`.Message` (break `BKActionDownloadRawFileOutput` _output_4)) 4.0)
          (goto _label_2))
        (:`Canceled`
          ;;;[1 0 0.09412] Download cancelled by user
          (`self.OnUpdateProgressCancelled` (`BlueprintMapLibrary.Map_Find` (`self.ActionIdFileId`) _actionid))
          (goto _label_2))))))

(event `OnDeleteFile`
  (params (ModelId :type String) (RevisionIndex :type Integer) (VersionIndex :type Integer) (NotifyUser :type Boolean))
  (bind _returnvalue (`BKManagerStore.GetNotificationManager`))
  ;[1 1 1] Delete file
  ;;[1 1 1] Create Action Id and Cancellation Token
  (bind _returnvalue_2 (`BKActionBase.GenerateActionId`))
  (set `self.LastActionId_DeleteFile` _returnvalue_2)
  (bind _returnvalue_3 (`|GenericCreateObject` "/BGenericAuthFileSrvClient/Blueprints/BP_BK_EmptyCancellationTokenObject.BP_BK_EmptyCancellationTokenObject_C" self))
  (bind _output (`/BGenericAuthFileSrvClient/Blueprints/BP_BK_EmptyCancellationTokenObject.SetRelevantToken` _returnvalue_3 (`BKCancellationToken.MakeFromUObject` _returnvalue_3)))
  (if NotifyUser
    (`BKNotificationManager.SendNotification` (`BKManagerStore.GetNotificationManager`) "Deleting file..." 6.0))
  (bind _output_2 (`BKActionDeleteFiles.Perform_DeleteFiles_Action_BP` (make `BKActionDeleteFilesInput` ModelId RevisionIndex VersionIndex (`self.LastActionId_DeleteFile`) true _output))
    (:`Succeed`
      ;;[0 1 0.007843] Succeeded
      (if NotifyUser
        (`BKNotificationManager.SendNotification` _returnvalue "File deleted" 4.0)))
    (:`Failed`
      ;;[1 0 0.09412] Failed
      (if NotifyUser
        (bind (_relativeinput _message) (break `BKActionDeleteFilesOutput` _output_2))
        (`BKNotificationManager.SendNotification` _returnvalue _message 4.0))))
  (bind _returnvalue_4 (`BKActionBlueprintFunctionLibrary.MakeFileId` (break `BKActionDeleteFilesInput` _relativeinput) (`.RevisionIndex` (break `BKActionDeleteFilesInput` _relativeinput)) (`.VersionIndex` (break `BKActionDeleteFilesInput` _relativeinput))))
  (`self.OnDeleteFilesEnd` _returnvalue_4)
  (`self.Add File for Retry State` _returnvalue_4))

(event `OnCancelFileOperation`
  (params (FileIdentifier :type String) (IsUpload :type Boolean))
  (bind (_lefts _rights) (`KismetStringLibrary.Split` FileIdentifier ":"))
  (bind _returnvalue (`BKManagerStore.GetNotificationManager`))
  (bind (_lefts_2 _rights_2) (`KismetStringLibrary.Split` _rights ":"))
  (bind (_value _returnvalue_2) (`BlueprintMapLibrary.Map_Find` (`self.FileIdCancellationTokenObjectMap`) FileIdentifier))
  ;[1 1 1] Cancel file operation
  (if _returnvalue_2
    (`BKCancellationToken.ForceKill` (`/BGenericAuthFileSrvClient/Blueprints/BP_BK_EmptyCancellationTokenObject.GetRelevantToken` _value))
    (`BlueprintMapLibrary.Map_Remove` (`self.FileIdCancellationTokenObjectMap`) FileIdentifier)
    (`BKNotificationManager.SendNotification` _returnvalue "File operation cancelled" 4.0)
    (if IsUpload
      (`self.OnDeleteFile` _lefts (`KismetStringLibrary.Conv_StringToInt` _lefts_2) (`KismetStringLibrary.Conv_StringToInt` _rights_2)))
    (else
      (`BKNotificationManager.SendNotification` _returnvalue "No current file operation" 4.0))))

(event `self.OnDestructBP`)

(event `OnAuthenticationStatusLost`
  (bind _fileidcancellationtokenobjectmap (`self.FileIdCancellationTokenObjectMap`))
  ;[1 1 1] Authentication status lost
  (if (> (`BlueprintMapLibrary.Map_Length` _fileidcancellationtokenobjectmap) 0)
    (bind _values (`BlueprintMapLibrary.Map_Values` _fileidcancellationtokenobjectmap))
    (for _array_element _values
      (`BKCancellationToken.ForceKill` (`/BGenericAuthFileSrvClient/Blueprints/BP_BK_EmptyCancellationTokenObject.GetRelevantToken` _array_element)))
    (`BlueprintMapLibrary.Map_Clear` (`self.FileIdCancellationTokenObjectMap`))
    (`BKNotificationManager.SendNotification` (`BKManagerStore.GetNotificationManager`) "Authentication status lost. All file processes cancelled" 6.0)))

(event `self.OnFirstTimeMapLoadedBP`)

(event `self.OnNonFirstTimeMapLoadedBP`)

(event `self.OnConstructBP`)

(event `self.OnBTick`
  (params (DeltaTime :type "Float (single-precision)"))
  ;[1 1 1] Tick (Only ticks when FileIdFileEntryRetries map is populated)
  (bind _keys (`BlueprintMapLibrary.Map_Keys` (`self.FileIdFileEntryRetries`)))
  (bind (_arrayindex _arrayelement) (`/Engine/EditorBlueprintResources/StandardMacros.ReverseForEachLoop` _keys)
    (:`LoopBody`
      (bind (_numberofretries _timetilltick _expectedstate) (break `/BGenericAuthFileSrvClient/Blueprints/BP_BK_GetFileEntryRetriesStruct` (`BlueprintMapLibrary.Map_Find` (`self.FileIdFileEntryRetries`) _arrayelement)))
      ;;[1 1 1] Remove entry if out of retries
      (if (== _numberofretries 0)
        (`self.RemoveFileForRetryState` _arrayelement)
        (`self.OnFinishForcefully` _arrayelement)
        (elif (> _timetilltick 0.0)
          ;;[1 1 1] Increment timer
          (`BlueprintMapLibrary.Map_Add` (`self.FileIdFileEntryRetries`) _arrayelement (make `/BGenericAuthFileSrvClient/Blueprints/BP_BK_GetFileEntryRetriesStruct` _numberofretries (- _timetilltick DeltaTime) _expectedstate))
          (else
            ;;[1 1 1] Retry
            (`BlueprintMapLibrary.Map_Add` (`self.FileIdFileEntryRetries`) _arrayelement (make `/BGenericAuthFileSrvClient/Blueprints/BP_BK_GetFileEntryRetriesStruct` (- _numberofretries 1) 3.0 _expectedstate))
            (bind (_lefts _rights) (`KismetStringLibrary.Split` _arrayelement ":"))
            (bind (_lefts_2 _rights_2) (`KismetStringLibrary.Split` _rights ":"))
            (`self.OnPerformGetVersionFileEntry` _lefts (`KismetStringLibrary.Conv_StringToInt` _lefts_2) (`KismetStringLibrary.Conv_StringToInt` _rights_2))))))))

(event `OnPerformGetVersionFileEntry`
  (params (ModelId :type String) (RevisionIndex :type Integer) (VersionIndex :type Integer))
  (bind _returnvalue (`|GenericCreateObject` "/BGenericAuthFileSrvClient/Blueprints/BP_BK_EmptyCancellationTokenObject.BP_BK_EmptyCancellationTokenObject_C" self))
  (bind _output (`/BGenericAuthFileSrvClient/Blueprints/BP_BK_EmptyCancellationTokenObject.SetRelevantToken` _returnvalue (`BKCancellationToken.MakeFromUObject` _returnvalue)))
  (bind _returnvalue_2 (`BKActionBase.GenerateActionId`))
  (bind _output_2 (`BKActionGetRevisionVersionInfo.Perform_GetRevisionVersionInfo_Action_BP` (make `BKActionGetRevisionVersionInfoInput` ModelId RevisionIndex VersionIndex _returnvalue_2 true _output))
    (:`Succeed`
      (bind (_modelid _revisionindex _versionindex) (break `BKActionGetRevisionVersionInfoInput` (break `BKActionGetRevisionVersionInfoOutput` _output_2)))
      (bind _returnvalue_3 (`BKActionBlueprintFunctionLibrary.MakeFileId` _modelid _revisionindex _versionindex))
      (if (== (`.ExpectedState_4_C4B2F4494ADDDC262F1200B77A0F0AC9` (break `/BGenericAuthFileSrvClient/Blueprints/BP_BK_GetFileEntryRetriesStruct` (`BlueprintMapLibrary.Map_Find` (`self.FileIdFileEntryRetries`) _returnvalue_3))) (`.fileProcessStage` (break `VersionFileEntry` (`.versionFileEntry` (break `ModelRevisionVersion` (`.Version` (break `BKActionGetRevisionVersionInfoOutput` _output_2)))))))
        (`self.RemoveFileForRetryState` _returnvalue_3)
        (`self.OnFileOperationSucceeded` _returnvalue_3)))))

(fn `Add File for Retry State`
  (params (FileId :type String) (ExpectedState :type Integer))
  (`BlueprintMapLibrary.Map_Add` (`self.FileIdFileEntryRetries`) FileId (make `/BGenericAuthFileSrvClient/Blueprints/BP_BK_GetFileEntryRetriesStruct` 10 3.0 (`KismetMathLibrary.Clamp` ExpectedState 0 2)))
  (`self.SetIsTickable` (> (`BlueprintMapLibrary.Map_Length` (`self.FileIdFileEntryRetries`)) 0)))

(fn `RemoveFileForRetryState`
  (params (FileId :type String))
  (`BlueprintMapLibrary.Map_Remove` (`self.FileIdFileEntryRetries`) FileId)
  (`self.SetIsTickable` (> (`BlueprintMapLibrary.Map_Length` (`self.FileIdFileEntryRetries`)) 0)))